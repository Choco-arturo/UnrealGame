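; AI controller for BP_AI pawns that runs a behavior tree and tells it when the player is in sight.
; When PawnSensing sees a BP_ThirdPersonCharacter, it writes the CanSeePlayer flag and PlayerTarget to the Blackboard.
; A retriggerable delay of twice the sensing interval acts as a lost-sight timeout, clearing the flag and stopping the pawn's Narunnig montage.
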(event `self.ReceiveBeginPlay`
  (`self.RunBehaviorTree` (`self.AI_BehaviorTree`))
  (bind _asbp_ai (cast `/Game/Arturo/AI/BP_AI` (`self.K2_GetPawn`)))
  (set `self.BPEnemy` _asbp_ai))

(event `self.PawnSensing.OnSeePawn`
  (params (Pawn :type "Pawn Object Reference"))
  (bind _asbp_third_person_character (cast `/Game/ThirdPerson/Blueprints/BP_ThirdPersonCharacter` Pawn))
  (`self.SetCanSeePlayer` true _asbp_third_person_character)
  (`KismetSystemLibrary.RetriggerableDelay` (* (`PawnSensingComponent.SensingInterval` (`self.PawnSensing`)) 2.0))
  (`self.SetCanSeePlayer` false)
  (`AnimInstance.Montage_Stop` (`SkeletalMeshComponent.GetAnimInstance` (`Character.Mesh` (`self.BPEnemy`))) 0.0 "/Game/Arturo/Player/Animations/Narunnig.Narunnig"))

(fn `SetCanSeePlayer`
  (params (CanSeePlayer :type Boolean) (PlayerObject :type "Object Object Reference"))
  (bind _returnvalue (`AIBlueprintHelperLibrary.GetBlackboard` self))
  (if CanSeePlayer
    (`BlackboardComponent.SetValueAsBool` _returnvalue "CanSeePlayer" true)
    (`BlackboardComponent.SetValueAsObject` _returnvalue "PlayerTarget" PlayerObject)
    (else
      (`BlackboardComponent.SetValueAsBool` _returnvalue "CanSeePlayer" false))))

(fn `UserConstructionScript`)