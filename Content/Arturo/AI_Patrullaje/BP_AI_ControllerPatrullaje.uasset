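; AI controller for a patrolling dog (BP_AI_Patrullaje) that runs BT_AI_Patrullaje on possession.
; On possess it gathers TargetPoints tagged "Dog"; GetNewPoint writes a random one to the blackboard's TargetPointKey.
; Walk and Run events forward to the possessed dog.
; Perception updates from the third-person character always set CanSeePlayer to false, and the PawnSensing handler is empty.
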(event `Walk`
  (`/Game/Arturo/AI_Patrullaje/BP_AI_Patrullaje.Walk` (`self.Perro`)))

(event `Run`
  (`/Game/Arturo/AI_Patrullaje/BP_AI_Patrullaje.Run` (`self.Perro`)))

(event `self.ReceivePossess`
  (params (PossessedPawn :type "Pawn Object Reference"))
  (bind _asbp_ai_patrullaje (cast `/Game/Arturo/AI_Patrullaje/BP_AI_Patrullaje` PossessedPawn))
  (set `self.Perro` _asbp_ai_patrullaje)
  (`self.RunBehaviorTree` "/Game/Arturo/AI_Patrullaje/BT_AI_Patrullaje.BT_AI_Patrullaje")
  (bind _outactors (`GameplayStatics.GetAllActorsOfClass` "/Script/Engine.TargetPoint"))
  (for _array_element _outactors
    (if (`self.ActorHasTag` _array_element "Dog")
      (`KismetArrayLibrary.Array_Add` (`self.PatrolPoints`) _array_element))))

(event `self.AIPerception.OnTargetPerceptionUpdated`
  (params (Actor :type "Actor Object Reference") (Stimulus :type "AIStimulus Structure"))
  (cast `/Game/ThirdPerson/Blueprints/BP_ThirdPersonCharacter` Actor)
  (`BlackboardComponent.SetValueAsBool` (`AIBlueprintHelperLibrary.GetBlackboard` null) "CanSeePlayer" false))

(event `GetNewPoint`
  (bind _patrolpoints (`self.PatrolPoints`))
  (`BlackboardComponent.SetValueAsObject` (`AIBlueprintHelperLibrary.GetBlackboard` null) "TargetPointKey" (`|GetArrayItem` _patrolpoints (`KismetMathLibrary.RandomIntegerInRange` 0 (- (`KismetArrayLibrary.Array_Length` _patrolpoints) 1)))))

(event `self.PawnSensing.OnSeePawn`
  (params (Pawn :type "Pawn Object Reference")))

(fn `UserConstructionScript`)