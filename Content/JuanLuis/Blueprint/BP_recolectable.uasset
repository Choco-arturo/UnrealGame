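; Collectible diamond pickup that counts toward advancing to Level2.
; When the third-person character overlaps its box, it plays sparks and a sound, increments the GameInstanceGefe counter and destroys itself.
; It also writes the count to the player save object and records itself in the level save object, both reached through the character's GameMode.
; At eight collected, it starts a camera fade and immediately opens Level2 by console command.
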(event `self.Box.OnComponentBeginOverlap`
  (params (OverlappedComponent :type "PrimitiveComponent Object Reference") (OtherActor :type "Actor Object Reference") (OtherComp :type "PrimitiveComponent Object Reference") (OtherBodyIndex :type Integer) (bFromSweep :type Boolean) (SweepResult :type "HitResult Structure (by ref)"))
  (bind _asbp_third_person_character (cast `/Game/ThirdPerson/Blueprints/BP_ThirdPersonCharacter` OtherActor))
  (bind _asgame_instance_gefe (cast `/Game/Gerardo/Vida/GameInstanceGefe` (`GameplayStatics.GetGameInstance`)))
  (`GameplayStatics.SpawnEmitterAtLocation` "/Game/StarterContent/Particles/P_Sparks.P_Sparks" (`self.K2_GetActorLocation`))
  (`GameplayStatics.PlaySoundAtLocation` "/Game/Gerardo/LevelSounds/MM_Notebook.MM_Notebook" (0.0 0.0 0.0) (struct) 1.0 1.0 0.0 null null null null)
  (bind _asbp_third_person_character_2 (cast `/Game/ThirdPerson/Blueprints/BP_ThirdPersonCharacter` OtherActor))
  (bind _returnvalue (+ (`/Game/Gerardo/Vida/GameInstanceGefe.RecolectablesGuardados` _asgame_instance_gefe) 1))
  (set `/Game/ThirdPerson/Blueprints/PlayerDataObject.DiamondPoints` _returnvalue (`/Game/ThirdPerson/Blueprints/BP_ThirdPersonGameMode.PlayerSaveObject` (`/Game/ThirdPerson/Blueprints/BP_ThirdPersonCharacter.GameMode` _asbp_third_person_character_2)))
  (bind _output_get (set `/Game/Gerardo/Vida/GameInstanceGefe.RecolectablesGuardados` _returnvalue _asgame_instance_gefe))
  (`KismetArrayLibrary.Array_AddUnique` (`/Game/ThirdPerson/Blueprints/LevelDataObject.DiamondsCollected` (`/Game/ThirdPerson/Blueprints/BP_ThirdPersonGameMode.LevelSaveObject` (`/Game/ThirdPerson/Blueprints/BP_ThirdPersonCharacter.GameMode` _asbp_third_person_character))) self)
  (`self.K2_DestroyActor`)
  (if (== _output_get 8)
    (`|ExecutionSequence`
      (:`then_0`
        (`PlayerCameraManager.StartCameraFade` :`self` (`GameplayStatics.GetPlayerCameraManager` 0) :`ToAlpha` 1.0 :`Duration` 5.0)
        (`KismetSystemLibrary.ExecuteConsoleCommand` "open Level2" null)))))

(fn `UserConstructionScript`)