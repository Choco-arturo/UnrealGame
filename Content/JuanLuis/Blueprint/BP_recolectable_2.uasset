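; BP_recolectable_2 is a Gorman mask collectible that the third-person character picks up by overlapping its Box.
; Pickup spawns a fire effect, plays a sound at world origin, increments the game instance's Recolectables2Guardados counter and destroys the actor.
; It also sets GormanMaskPoints to zero in the player save object and records itself in the level save's GormanMasksCollected.
; An unconnected fade-out and Level3 load never runs.
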(event `self.Box.OnComponentBeginOverlap`
  (params (OverlappedComponent :type "PrimitiveComponent Object Reference") (OtherActor :type "Actor Object Reference") (OtherComp :type "PrimitiveComponent Object Reference") (OtherBodyIndex :type Integer) (bFromSweep :type Boolean) (SweepResult :type "HitResult Structure (by ref)"))
  (bind _asbp_third_person_character (cast `/Game/ThirdPerson/Blueprints/BP_ThirdPersonCharacter` OtherActor))
  (bind _asgame_instance_gefe (cast `/Game/Gerardo/Vida/GameInstanceGefe` (`GameplayStatics.GetGameInstance`)))
  (`GameplayStatics.SpawnEmitterAtLocation` "/Game/StarterContent/Particles/P_Fire.P_Fire" (`self.K2_GetActorLocation`))
  (`GameplayStatics.PlaySoundAtLocation` "/Game/Gerardo/LevelSounds/OOT_Ingo_Yell.OOT_Ingo_Yell" (0.0 0.0 0.0) (struct) 1.0 1.0 0.0 null null null null)
  (bind _asbp_third_person_character_2 (cast `/Game/ThirdPerson/Blueprints/BP_ThirdPersonCharacter` OtherActor))
  (set `/Game/ThirdPerson/Blueprints/PlayerDataObject.GormanMaskPoints` 0 (`/Game/ThirdPerson/Blueprints/BP_ThirdPersonGameMode.PlayerSaveObject` (`/Game/ThirdPerson/Blueprints/BP_ThirdPersonCharacter.GameMode` _asbp_third_person_character_2)))
  (set `/Game/Gerardo/Vida/GameInstanceGefe.Recolectables2Guardados` (+ (`/Game/Gerardo/Vida/GameInstanceGefe.Recolectables2Guardados` _asgame_instance_gefe) 1) _asgame_instance_gefe)
  (`KismetArrayLibrary.Array_AddUnique` (`/Game/ThirdPerson/Blueprints/LevelDataObject.GormanMasksCollected` (`/Game/ThirdPerson/Blueprints/BP_ThirdPersonGameMode.LevelSaveObject` (`/Game/ThirdPerson/Blueprints/BP_ThirdPersonCharacter.GameMode` _asbp_third_person_character))) self)
  (`self.K2_DestroyActor`))

(fn `UserConstructionScript`)